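; BP_IcicleVolume is a box volume that rains icicles at random, spaced-out spots beneath it while active.
; StartIcicleSpawns clears saved locations and starts a looping timer, which StopIcicleSpawns cancels.
; Each tick traces downward between random box points, retrying without limit until a hit passes a proximity check against every location saved that run.
; Accepted hits are saved, then get a BP_Telegraph_Icicle marker and a scaled-up BP_Icicle spawned high above.
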(event `StartIcicleSpawns`
  ;[1 1 1] Start Timer
  (`KismetArrayLibrary.Array_Clear` (`self.ArrayOfIcicleLocs`))
  (bind _returnvalue (`KismetSystemLibrary.K2_SetTimerDelegate` (delegate `FindSpawnLoc`) 0.25 true))
  (set `self.IcicleSpawnTimer` _returnvalue))

(event `FindSpawnLoc`
  (bind _returnvalue (`KismetMathLibrary.RandomPointInBoundingBox` (`self.K2_GetActorLocation`) (`BoxComponent.GetScaledBoxExtent` (`self.IcicleVolume`))))
  (bind _outhit (`KismetSystemLibrary.LineTraceSingleForObjects` _returnvalue (- _returnvalue (0.0 0.0 2000.0)) (`|MakeArray` "ObjectTypeQuery8" :!type "EObjectTypeQuery Enum") :!label _label))
  (bind (_bblockinghit _binitialoverlap _time _distance _location) (`GameplayStatics.BreakHitResult` _outhit))
  (if _bblockinghit
    (if (== (`KismetArrayLibrary.Array_Length` (`self.ArrayOfIcicleLocs`)) 0)
      (`KismetArrayLibrary.Array_Add` (`self.ArrayOfIcicleLocs`) _location)
      (else
        (for _array_element (`self.ArrayOfIcicleLocs`)
          (if (== _location (`KismetMathLibrary.MakeVector` (.x _array_element) (.y _array_element)) :`ErrorTolerance` 400.0)
            (set `self.InvalidIcicleLoc` true)
            (break)))
        (if (`self.InvalidIcicleLoc`)
          (set `self.InvalidIcicleLoc` false)
          (goto _label)
          (else
            (`KismetArrayLibrary.Array_Add` (`self.ArrayOfIcicleLocs`) _location)))))
    (`|SpawnActorFromClass` "/Game/Blueprints/BP_Telegraph_Icicle.BP_Telegraph_Icicle_C" (`KismetMathLibrary.MakeTransform` _location) "Undefined" "OverrideRootScale" null null)
    (`|SpawnActorFromClass` "/Game/Assets/Meshes/BP_Icicle.BP_Icicle_C" (`KismetMathLibrary.MakeTransform` (+ _location (0.0 0.0 2500.0)) (struct) (4.0 4.0 4.0)) "Undefined" "OverrideRootScale" null null)
    (else
      (goto _label))))

(event `StopIcicleSpawns`
  ;[1 1 1] Stop Timer
  (`KismetSystemLibrary.K2_ClearAndInvalidateTimerHandle` (`self.IcicleSpawnTimer`)))

(fn `UserConstructionScript`)