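; BP_Icicle_OLD is a short-lived icicle hazard that damages the player on overlap.
; On spawn, its Cone has collision disabled briefly, then enabled, and the actor destroys itself a few seconds later.
; Overlapping a BP_Player_Parent calls its TakeDamage with a fixed amount and destroys the icicle immediately.
; A MoveComponentTo node for sliding the Cone is left unconnected and never runs.
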(event `self.ReceiveBeginPlay`
  (bind _cone (`self.Cone`))
  (`PrimitiveComponent.SetCollisionEnabled` _cone "NoCollision")
  (`KismetSystemLibrary.Delay` 0.25)
  (`PrimitiveComponent.SetCollisionEnabled` _cone "QueryAndPhysics")
  (`KismetSystemLibrary.Delay` 3.0)
  (`self.K2_DestroyActor`))

(event `self.ReceiveActorBeginOverlap`
  (params (OtherActor :type "Actor Object Reference"))
  (bind _asbp_player_parent (cast `/Game/Blueprints/Characters/BP_Player_Parent` OtherActor))
  (`/Game/Blueprints/Characters/BP_Player_Parent.TakeDamage` _asbp_player_parent 5.0)
  (`self.K2_DestroyActor`))

(fn `UserConstructionScript`)