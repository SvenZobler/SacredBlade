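; Cherry bomb actor for the Assassin character that explodes on a timer or on contact with the boss.
; After the detonation delay, a 300-unit sphere trace damages the boss and sets shurikens on fire.
; Overlapping a Boss-tagged actor deals separate direct-hit damage with a flash.
; Both paths spawn an explosion, grant ult charge through the instigating player and destroy the bomb.
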(event `self.ReceiveBeginPlay`
  (bind _returnvalue (`self.K2_GetActorLocation`))
  (bind _cherrybombdamage (`self.CherryBombDamage`))
  (`KismetSystemLibrary.Delay` (`self.DetonationTimer`))
  (`GameplayStatics.SpawnEmitterAtLocation` "/Game/Explosions/Particles/P_ImpactExplosion4.P_ImpactExplosion4" _returnvalue)
  (bind _outhits (`KismetSystemLibrary.SphereTraceMultiForObjects` _returnvalue (+ _returnvalue (0.0 0.0 0.1)) 300.0 (`|MakeArray` "ObjectTypeQuery2" :!type "EObjectTypeQuery Enum")))
  (for _array_element _outhits
    (bind (_bblockinghit _binitialoverlap _time _distance _location _impactpoint _normal _impactnormal _physmat _hitactor) (`GameplayStatics.BreakHitResult` _array_element))
    (bind _asbp_boss (cast `/Game/Blueprints/Characters/BP_Boss` _hitactor)
      (:`then`
        (bind _asbp_player_parent (cast `/Game/Blueprints/Characters/BP_Player_Parent` (`self.Instigator`))
          (:`then`
            (`/Game/Blueprints/Characters/BP_Player_Parent.AddUltCharge` _asbp_player_parent _cherrybombdamage)
            (`/Game/Blueprints/Characters/BP_Boss.TakeDamage` _asbp_boss _cherrybombdamage)
            (bind _asbp_shuriken (cast `/Game/Blueprints/Characters/Assassin/BP_Shuriken` _hitactor :!label _label)
              (:`then`
                (`/Game/Blueprints/Characters/Assassin/BP_Shuriken.SetOnFire` _asbp_shuriken))
              (:`CastFailed`
                _))
            (`self.K2_DestroyActor` :!label _label_2))
          (:`CastFailed`
            (`KismetSystemLibrary.PrintString` "Can't find parent"))))
      (:`CastFailed`
        (goto _label))))
  (goto _label_2))

(event `self.ReceiveActorBeginOverlap`
  (params (OtherActor :type "Actor Object Reference"))
  (bind _cherrybombdirectdamage (`self.CherryBombDirectDamage`))
  (`/Engine/EditorBlueprintResources/StandardMacros.IsValid` OtherActor
    (:`Is Valid`
      (if (`self.ActorHasTag` OtherActor "Boss")
        (`GameplayStatics.SpawnEmitterAtLocation` "/Game/Explosions/Particles/P_ImpactExplosion4.P_ImpactExplosion4" (`self.K2_GetActorLocation`))
        (bind _asbp_boss (cast `/Game/Blueprints/Characters/BP_Boss` OtherActor))
        ;[1 1 1] Damage Feedback
        (`/Game/Blueprints/Characters/BP_Boss.DamageFlash` _asbp_boss)
        ;[1 1 1] Add Ult Charge
        (bind _asbp_player_parent (cast `/Game/Blueprints/Characters/BP_Player_Parent` (`self.Instigator`))
          (:`then`
            (`/Game/Blueprints/Characters/BP_Player_Parent.AddUltCharge` _asbp_player_parent _cherrybombdirectdamage))
          (:`CastFailed`
            _))
        ;[1 1 1] TakeDamage
        (`/Game/Blueprints/Characters/BP_Boss.TakeDamage` _asbp_boss _cherrybombdirectdamage)
        (`self.K2_DestroyActor`)))))

(fn `UserConstructionScript`)