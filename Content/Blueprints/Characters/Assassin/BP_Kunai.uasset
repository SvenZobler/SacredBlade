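; BP_Kunai is the Assassin's kunai projectile, which damages bosses on contact.
; On overlapping an actor tagged Boss, it casts to BP_Boss, triggers a damage flash, applies KunaiDamage and destroys itself.
; If the instigator is a BP_Player_Parent, the same damage value also adds to that player's ultimate charge.
; The ProjectileEffect event is empty, and construction defers to the parent script.
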(event `self.ProjectileEffect`)

(event `self.ReceiveActorBeginOverlap`
  (params (OtherActor :type "Actor Object Reference"))
  (bind _kunaidamage (`self.KunaiDamage`))
  (if (`self.ActorHasTag` OtherActor "Boss")
    (bind _asbp_boss (cast `/Game/Blueprints/Characters/BP_Boss` OtherActor))
    (`/Game/Blueprints/Characters/BP_Boss.DamageFlash` _asbp_boss)
    (bind _asbp_player_parent (cast `/Game/Blueprints/Characters/BP_Player_Parent` (`self.Instigator`))
      (:`then`
        (`/Game/Blueprints/Characters/BP_Player_Parent.AddUltCharge` _asbp_player_parent _kunaidamage))
      (:`CastFailed`
        _))
    (`/Game/Blueprints/Characters/BP_Boss.TakeDamage` _asbp_boss _kunaidamage)
    (`self.K2_DestroyActor`)))

(fn `UserConstructionScript`
  (`parent.UserConstructionScript`))