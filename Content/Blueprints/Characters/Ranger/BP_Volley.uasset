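; BP_Volley is a short-lived Ranger volley actor that displays a scattered cluster of arrows.
; On BeginPlay, VisibleArrows selects one of three tiers, each revealing a progressively larger set of arrow components.
; Each handled tier then gives every arrow a random local rotation within fixed limits, and the actor destroys itself after a brief delay.
; The graph contains no movement or damage logic.
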(event `self.ReceiveBeginPlay`
  (switch `int` (`self.VisibleArrows`)
    (:`3`
      (`SceneComponent.SetVisibility` (`self.arrow2`) true false)
      (`SceneComponent.SetVisibility` (`self.arrow1`) true false)
      (`SceneComponent.SetVisibility` (`self.arrow3`) true false)
      (`SceneComponent.SetVisibility` (`self.arrow`) true false))
    (:`4`
      (`SceneComponent.SetVisibility` (`self.arrow1`) true false)
      (`SceneComponent.SetVisibility` (`self.arrow2`) true false)
      (`SceneComponent.SetVisibility` (`self.arrow3`) true false)
      (`SceneComponent.SetVisibility` (`self.arrow4`) true false)
      (`SceneComponent.SetVisibility` (`self.arrow5`) true false)
      (`SceneComponent.SetVisibility` (`self.arrow`) true false))
    (:`5`
      (`SceneComponent.SetVisibility` (`self.arrow5`) true false)
      (`SceneComponent.SetVisibility` (`self.arrow4`) true false)
      (`SceneComponent.SetVisibility` (`self.arrow3`) true false)
      (`SceneComponent.SetVisibility` (`self.arrow2`) true false)
      (`SceneComponent.SetVisibility` (`self.arrow1`) true false)
      (`SceneComponent.SetVisibility` (`self.arrow6`) true false)
      (`SceneComponent.SetVisibility` (`self.arrow7`) true false)
      (`SceneComponent.SetVisibility` (`self.arrow`) true false)))
  (`self.Rotations`)
  (`KismetSystemLibrary.Delay` 1.5)
  (`self.K2_DestroyActor`))

(fn `RandomRotation`
  (params (self2 :type "SceneComponent Object Reference"))
  (`SceneComponent.K2_AddLocalRotation` self2 (`KismetMathLibrary.MakeRotator` (`KismetMathLibrary.RandomFloatInRange` -30.0 30.0) (`KismetMathLibrary.RandomFloatInRange` -40.0 40.0) (`KismetMathLibrary.RandomFloatInRange` -15.0 15.0)) false false))

(fn `Rotations`
  (`self.RandomRotation` (`self.arrow1`))
  (`self.RandomRotation` (`self.arrow2`))
  (`self.RandomRotation` (`self.arrow3`))
  (`self.RandomRotation` (`self.arrow`))
  (`self.RandomRotation` (`self.arrow5`))
  (`self.RandomRotation` (`self.arrow6`))
  (`self.RandomRotation` (`self.arrow7`))
  (`self.RandomRotation` (`self.arrow4`)))

(fn `UserConstructionScript`)