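; Wizard player character with a repeating bolt shot, a cooldown fireball and a charge-gated Arcane Beam ultimate.
; BeginPlay loads stats from T_WizardVars, caches the boss and pre-spawns hidden beam emitters.
; Timers drive held fire and fireball cooldown, though bolt rate and beam length use hardcoded values instead of table stats.
; The beam toggles emitter visibility and runs a looping box trace that damages the Boss-tagged target until BeamDuration ends.
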(event `self.ReceiveTick`
  (params (DeltaSeconds :type "Float (single-precision)")))

(event `self.ReceiveBeginPlay`
  ;[1 1 1] Setup/Var Get
  (`self.SpawnFunction`)
  (`self.BeamHitSetup`)
  (`self.BeamSetup`)
  (bind _returnvalue (`|GetDataTableRow` "/Game/Blueprints/Characters/Wizard/T_WizardVars.T_WizardVars" "BaseStats")
    (:`then`
      (bind (_boltdamage _boltspeed _boltrateoffire _fireballdamage _fireballfirepatchdamage _fireballfirepatchduration _fireballcooldown _beamdamage _beamlength _beamduration) (break `/Game/Blueprints/Characters/Wizard/S_WizardVars` _returnvalue))
      (set `self.BoltDamage` _boltdamage)
      (set `self.BoltSpeed` _boltspeed)
      (set `self.BoltRateofFire` _boltrateoffire)
      (set `self.FireballDamage` _fireballdamage)
      (set `self.FireballPatchDuration` _fireballfirepatchduration)
      (set `self.FireballPatchDamage` _fireballfirepatchdamage)
      (set `self.FireballCooldown` _fireballcooldown)
      (set `self.BeamDamage` _beamdamage)
      (set `self.BeamLength` _beamlength)
      (set `self.BeamDuration` _beamduration)
      (bind _outactors (`GameplayStatics.GetAllActorsOfClass` "/Game/Blueprints/Characters/BP_Boss.BP_Boss_C"))
      (set `self.REFBoss` (`|GetArrayItem` _outactors)))))

(event `RateofFireClock`
  ;[1 1 1] BoltTimer
  (`KismetSystemLibrary.K2_SetTimerDelegate` (delegate `RateofFireBoolSetter`) 0.49 true))

(event `RateofFireBoolSetter`
  ;[1 1 1] BoltTimer
  (set `self.CanFire` true))

(event `InputAction|Shoot`
  (params (Key :type "Key Structure"))
  ;[1 1 1] Bolt
  (:`Pressed`
    (if (`self.CanFire`)
      (set `self.CanFire` false)
      (`self.RateofFireClock`)
      (`self.BoltProj`))
    (bind _returnvalue (`KismetSystemLibrary.K2_SetTimerDelegate` (delegate `self.ShootFunction`) 0.5 true)))
  (:`Released`
    (`KismetSystemLibrary.K2_ClearAndInvalidateTimerHandle` _returnvalue)))

(event `self.ShootFunction`
  ;[1 1 1] Bolt
  (`self.BoltProj`))

(event `FireballStartTimer`
  ;[1 1 1] FireballCD
  (set `self.FireballReady` false)
  (`KismetSystemLibrary.K2_SetTimerDelegate` (delegate `CherryBombCDTimer`) (`self.FireballCooldown`)))

(event `InputAction|BasicAbility`
  (params (Key :type "Key Structure"))
  (bind (_returnvalue_location _returnvalue_rotation) (`KismetMathLibrary.BreakTransform` (`SceneComponent.K2_GetComponentToWorld` (`self.ProjSpawnLoc`))))
  ;[1 1 1] Fireball
  (:`Pressed`
    (if (`self.FireballReady`)
      (set `self.FireballReady` false)
      (`self.FireballStartTimer`)
      (`|SpawnActorFromClass` "/Game/Blueprints/Characters/Wizard/BP_Fireball.BP_Fireball_C" (`KismetMathLibrary.MakeTransform` _returnvalue_location _returnvalue_rotation (3.0 3.0 3.0)) "Undefined" "OverrideRootScale" null (`self.FireballDamage`) (`self.FireballPatchDamage`) self))))

(event `CherryBombCDTimer`
  ;[1 1 1] FireballCD
  (set `self.FireballReady` true))

(event `InputAction|UltimateAbility`
  (params (Key :type "Key Structure"))
  ;[1 1 1] Arcane Beam
  (:`Pressed`
    (if (== (`self.CurrentUltCharge`) (`self.UltChargeRequired`))
      (`self.BeamStart`)
      (set `self.CurrentUltCharge` 0.0)
      (set `self.NormalizedUltCharge` 0.0))))

(event `StopBeam`
  ;[1 1 1] Arcane Beam
  (`SceneComponent.SetVisibility` (`self.REFBeamEmitter`) false false)
  (`SceneComponent.SetVisibility` (`self.REFBeamHit`) false false)
  (`KismetSystemLibrary.K2_ClearAndInvalidateTimerHandle` (stale `BeamStart` _returnvalue)))

(event `BeamStart`
  ;[1 1 1] Arcane Beam
  (`SceneComponent.SetVisibility` (`self.REFBeamHit`) true false)
  (`SceneComponent.SetVisibility` (`self.REFBeamEmitter`) true false)
  (bind _returnvalue (`KismetSystemLibrary.K2_SetTimerDelegate` (delegate `BeamDamageTimer`) 0.1 true))
  (`KismetSystemLibrary.K2_SetTimer` null "StopBeam" (`self.BeamDuration`)))

(event `BeamDamageTimer`
  (bind _arrow1 (`self.Arrow1`))
  (bind _refboss (`self.REFBoss`))
  (bind _returnvalue (`SceneComponent.K2_GetComponentLocation` _arrow1))
  ;[1 1 1] Arcane Beam
  (bind _outhit (`KismetSystemLibrary.BoxTraceSingleForObjects` _returnvalue (+ _returnvalue (* (`SceneComponent.GetForwardVector` _arrow1) 2000.0)) (25.0 25.0 25.0) (struct) (`|MakeArray` "ObjectTypeQuery7" :!type "EObjectTypeQuery Enum")))
  (bind (_bblockinghit _binitialoverlap _time _distance _location _impactpoint _normal _impactnormal _physmat _hitactor) (`GameplayStatics.BreakHitResult` _outhit))
  (`/Engine/EditorBlueprintResources/StandardMacros.IsValid` _hitactor
    (:`Is Valid`
      (if (`self.ActorHasTag` _hitactor "Boss")
        (`/Game/Blueprints/Characters/BP_Boss.DamageFlash` _refboss)
        (`/Game/Blueprints/Characters/BP_Boss.TakeDamage` _refboss (`self.BeamDamage`))))))

(fn `BeamHitSetup`
  (bind _projspawnloc (`self.ProjSpawnLoc`))
  (bind _returnvalue (`GameplayStatics.SpawnEmitterAttached` "/Game/Stylized_FX5/ParticleSystems/Energy_Beam/P_ArcaneBeam_Hit.P_ArcaneBeam_Hit" _projspawnloc "None" (+ (`SceneComponent.K2_GetComponentLocation` _projspawnloc) (2000.0 0.0 0.0)) (struct) (1.0 1.0 1.0) "KeepWorldPosition"))
  (bind _output_get (set `self.REFBeamHit` _returnvalue))
  (`SceneComponent.SetVisibility` _output_get false false))

(fn `BeamSetup`
  (bind _projspawnloc (`self.ProjSpawnLoc`))
  (bind _returnvalue (`GameplayStatics.SpawnEmitterAttached` "/Game/Stylized_FX5/ParticleSystems/Energy_Beam/P_ArcaneBeam.P_ArcaneBeam" _projspawnloc "None" (`SceneComponent.K2_GetComponentLocation` _projspawnloc) (struct) (1.0 1.0 1.0) "KeepWorldPosition"))
  (bind _output_get (set `self.REFBeamEmitter` _returnvalue))
  (`SceneComponent.SetVisibility` _output_get false false))

(fn `BoltProj`
  (bind (_returnvalue_location _returnvalue_rotation) (`KismetMathLibrary.BreakTransform` (`SceneComponent.K2_GetComponentToWorld` (`self.ProjSpawnLoc`))))
  (`|SpawnActorFromClass` "/Game/Blueprints/Characters/Wizard/BP_Bolt.BP_Bolt_C" (`KismetMathLibrary.MakeTransform` _returnvalue_location _returnvalue_rotation) "Undefined" "OverrideRootScale" null (`self.BoltDamage`) self))

(fn `UserConstructionScript`
  (`parent.UserConstructionScript`))