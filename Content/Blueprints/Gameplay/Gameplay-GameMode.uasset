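; Gameplay game mode for a local multiplayer boss fight that spawns up to four player characters and manages their HUD.
; On BeginPlay it reads the player count from the game instance, creates players, possesses fixed classes by index, and creates boss-health and victory widgets.
; Per-player events add health and ultimate bars after a delay.
; Separate events swap pawns (alternating Wizard/Assassin, or back to InitPawn) and display victory; spawn-point gathering is disconnected.
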(event `self.ReceiveBeginPlay`
  (bind _returnvalue (`GameplayStatics.GetPlayerController` 0))
  (set `self.InstancePlayerCount` (`/Game/Blueprints/Gameplay/BP_GameInstance.PlayerCount` (cast `/Game/Blueprints/Gameplay/BP_GameInstance` (`GameplayStatics.GetGameInstance`) :!pure true)))
  (`self.SpawnPlayers`)
  (bind _returnvalue_2 (`|CreateWidget` "/Game/UI/Widgets/W_VictoryTemp.W_VictoryTemp_C" _returnvalue))
  (set `self.W_Victory` _returnvalue_2)
  (bind _returnvalue_3 (`|CreateWidget` "/Game/UI/Widgets/W_BossHealthBar.W_BossHealthBar_C" _returnvalue))
  (`UserWidget.AddToViewport` _returnvalue_3 0))

(event `SpawnCharacter`
  (params (`Player Controller` :type "PlayerController Object Reference"))
  (bind _returnvalue (`Controller.K2_GetPawn` `Player Controller`))
  (bind _asgameplayer__player_controller (cast `/Game/Blueprints/Gameplay/Gameplayer-PlayerController` `Player Controller` :!pure true))
  (bind _returnvalue_2 (`self.GetTransform`))
  (bind _gamecamera (`self.GameCamera`))
  (`/Engine/EditorBlueprintResources/StandardMacros.IsValid` _returnvalue
    (:`Is Valid`
      (`self.K2_DestroyActor` _returnvalue)
      (`/Engine/EditorBlueprintResources/StandardMacros.FlipFlop`
        (:`A`
          (bind _returnvalue_3 (`|SpawnActorFromClass` "/Game/Blueprints/Characters/Wizard/BP_Player_Wizard.BP_Player_Wizard_C" _returnvalue_2 "Undefined" "OverrideRootScale" null 0 null))
          (`Controller.Possess` `Player Controller` _returnvalue_3)
          (`PlayerController.SetViewTargetWithBlend` `Player Controller` _gamecamera 0.0 "VTBlend_Linear" 0.0 false)
          (`/Engine/EditorBlueprintResources/StandardMacros.IsValid` `Player Controller`
            (:`Is Valid`
              (`UserWidget.AddToViewport` (`/Game/Blueprints/Gameplay/Gameplayer-PlayerController.UltBarP1` _asgameplayer__player_controller) 0)
              (`UserWidget.AddToViewport` (`/Game/Blueprints/Gameplay/Gameplayer-PlayerController.HealthBarP1` _asgameplayer__player_controller) 0))))
        (:`B`
          (bind _returnvalue_4 (`|SpawnActorFromClass` "/Game/Blueprints/Characters/Assassin/BP_Player_Assassin.BP_Player_Assassin_C" _returnvalue_2 "Undefined" "OverrideRootScale" null 0 null))
          (`Controller.Possess` `Player Controller` _returnvalue_4)
          (`PlayerController.SetViewTargetWithBlend` `Player Controller` _gamecamera 0.0 "VTBlend_Linear" 0.0 false)
          (`UserWidget.AddToViewport` (`/Game/Blueprints/Gameplay/Gameplayer-PlayerController.HealthBarP2` _asgameplayer__player_controller) 0)
          (`UserWidget.AddToViewport` (`/Game/Blueprints/Gameplay/Gameplayer-PlayerController.UltBarP2` _asgameplayer__player_controller) 0))))))

(event `DespawnCharacter`
  (params (PlayerController :type "PlayerController Object Reference"))
  (bind _returnvalue (`Controller.K2_GetPawn` PlayerController))
  (`/Engine/EditorBlueprintResources/StandardMacros.IsValid` _returnvalue
    (:`Is Valid`
      (`self.K2_DestroyActor` _returnvalue)
      (bind _returnvalue_2 (`|SpawnActorFromClass` "/Game/Blueprints/Characters/InitPawn.InitPawn_C" (`self.GetTransform`) "Undefined" "OverrideRootScale" null null))
      (`Controller.Possess` PlayerController _returnvalue_2)
      (`PlayerController.SetViewTargetWithBlend` PlayerController (`self.GameCamera`) 0.0 "VTBlend_Linear" 0.0 false))))

(event `Victory`
  (`KismetSystemLibrary.Delay` 0.5)
  (`UserWidget.AddToViewport` (`self.W_Victory`) 0))

(event `Player1HUD`
  (params (PlayerController :type "PlayerController Object Reference"))
  ;[1 1 1] Setup Player HUD
  (`KismetSystemLibrary.Delay` 0.5)
  (bind _asgameplayer__player_controller (cast `/Game/Blueprints/Gameplay/Gameplayer-PlayerController` PlayerController))
  (`UserWidget.AddToViewport` (`/Game/Blueprints/Gameplay/Gameplayer-PlayerController.HealthBarP1` _asgameplayer__player_controller) 0)
  (`UserWidget.AddToViewport` (`/Game/Blueprints/Gameplay/Gameplayer-PlayerController.UltBarP1` _asgameplayer__player_controller) 0))

(event `Player2HUD`
  (params (PlayerController :type "PlayerController Object Reference"))
  ;[1 1 1] Setup Player HUD
  (`KismetSystemLibrary.Delay` 0.5)
  (bind _asgameplayer__player_controller (cast `/Game/Blueprints/Gameplay/Gameplayer-PlayerController` PlayerController))
  (`UserWidget.AddToViewport` (`/Game/Blueprints/Gameplay/Gameplayer-PlayerController.HealthBarP2` _asgameplayer__player_controller) 0)
  (`UserWidget.AddToViewport` (`/Game/Blueprints/Gameplay/Gameplayer-PlayerController.UltBarP2` _asgameplayer__player_controller) 0))

(event `Player3HUD`
  (params (PlayerController :type "PlayerController Object Reference"))
  ;[1 1 1] Setup Player HUD
  (`KismetSystemLibrary.Delay` 0.5)
  (bind _asgameplayer__player_controller (cast `/Game/Blueprints/Gameplay/Gameplayer-PlayerController` PlayerController))
  (`UserWidget.AddToViewport` (`/Game/Blueprints/Gameplay/Gameplayer-PlayerController.HealthBarP3` _asgameplayer__player_controller) 0)
  (`UserWidget.AddToViewport` (`/Game/Blueprints/Gameplay/Gameplayer-PlayerController.UltBarP3` _asgameplayer__player_controller) 0))

(event `Player4HUD`
  (params (PlayerController :type "PlayerController Object Reference"))
  ;[1 1 1] Setup Player HUD
  (`KismetSystemLibrary.Delay` 0.5)
  (bind _asgameplayer__player_controller (cast `/Game/Blueprints/Gameplay/Gameplayer-PlayerController` PlayerController))
  (`UserWidget.AddToViewport` (`/Game/Blueprints/Gameplay/Gameplayer-PlayerController.HealthBarP4` _asgameplayer__player_controller) 0)
  (`UserWidget.AddToViewport` (`/Game/Blueprints/Gameplay/Gameplayer-PlayerController.UltBarP4` _asgameplayer__player_controller) 0))

(fn `AddPlayerUIBars`
  (params (PlayerController :type "PlayerController Object Reference") (ControllerID :type Integer))
  (switch `int` ControllerID
    (:`0`
      (bind _asgameplayer__player_controller (cast `/Game/Blueprints/Gameplay/Gameplayer-PlayerController` PlayerController))
      (`UserWidget.AddToViewport` (`/Game/Blueprints/Gameplay/Gameplayer-PlayerController.HealthBarP1` _asgameplayer__player_controller) 0)
      (`UserWidget.AddToViewport` (`/Game/Blueprints/Gameplay/Gameplayer-PlayerController.UltBarP1` _asgameplayer__player_controller) 0))
    (:`1`
      (bind _asgameplayer__player_controller_2 (cast `/Game/Blueprints/Gameplay/Gameplayer-PlayerController` PlayerController))
      (`UserWidget.AddToViewport` (`/Game/Blueprints/Gameplay/Gameplayer-PlayerController.HealthBarP2` _asgameplayer__player_controller_2) 0)
      (`UserWidget.AddToViewport` (`/Game/Blueprints/Gameplay/Gameplayer-PlayerController.UltBarP2` _asgameplayer__player_controller_2) 0))))

(fn `DestroyInitPawn`
  (params (PlayerIndex :type Integer))
  (returns (ReturnValue :type "PlayerController Object Reference"))
  (bind _returnvalue (`GameplayStatics.GetPlayerController` PlayerIndex))
  (bind _returnvalue_2 (`Controller.K2_GetPawn` _returnvalue))
  (`/Engine/EditorBlueprintResources/StandardMacros.IsValid` _returnvalue_2
    (:`Is Valid`
      (`self.K2_DestroyActor` _returnvalue_2))
    (:`Is Not Valid`
      _))
  (return _returnvalue))

(fn `GetRandomPlayer`)

(fn `SpawnPlayers`
  (bind _returnvalue (`KismetMathLibrary.MakeTransform` (0.0 0.0 2000.0)))
  (for _ (range (+ (`self.InstancePlayerCount`) 1))
    (`GameplayStatics.CreatePlayer` -1))
  (for _index (range (+ (`self.InstancePlayerCount`) 1))
    (switch `int` _index
      (:`0`
        (bind _returnvalue_2 (`self.DestroyInitPawn` _index))
        (bind _returnvalue_3 (`|SpawnActorFromClass` "/Game/Blueprints/Characters/Ranger/BP_Player_Ranger.BP_Player_Ranger_C" _returnvalue "Undefined" "OverrideRootScale" null _index null))
        (`Controller.Possess` _returnvalue_2 _returnvalue_3)
        (`self.Player1HUD` _returnvalue_2))
      (:`1`
        (bind _returnvalue_4 (`self.DestroyInitPawn` _index))
        (bind _returnvalue_5 (`|SpawnActorFromClass` "/Game/Blueprints/Characters/Wizard/BP_Player_Wizard.BP_Player_Wizard_C" _returnvalue "Undefined" "OverrideRootScale" null _index null))
        (`Controller.Possess` _returnvalue_4 _returnvalue_5)
        (`self.Player2HUD` _returnvalue_4))
      (:`2`
        (bind _returnvalue_6 (`self.DestroyInitPawn` _index))
        (bind _returnvalue_7 (`|SpawnActorFromClass` "/Game/Blueprints/Characters/Ranger/BP_Player_Ranger.BP_Player_Ranger_C" _returnvalue "Undefined" "OverrideRootScale" null _index null))
        (`Controller.Possess` _returnvalue_6 _returnvalue_7)
        (`self.Player3HUD` _returnvalue_6))
      (:`3`
        (bind _returnvalue_8 (`self.DestroyInitPawn` _index))
        (bind _returnvalue_9 (`|SpawnActorFromClass` "/Game/Blueprints/Characters/Assassin/BP_Player_Assassin.BP_Player_Assassin_C" _returnvalue "Undefined" "OverrideRootScale" null _index null))
        (`Controller.Possess` _returnvalue_8 _returnvalue_9)
        (`self.Player4HUD` _returnvalue_8)))))

(fn `UserConstructionScript`)