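; Player controller for local gameplay that lets a player spawn or despawn their character and builds the four-player HUD widgets.
; On BeginPlay it caches the Gameplay game mode, then after a short delay creates and stores health and ult bar widgets for players one to four, without adding them to the viewport.
; Keyboard number keys or gamepad special buttons ask the game mode to spawn or despawn this controller's character.
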(event `self.ReceiveBeginPlay`
  (bind _asgameplay__game_mode (cast `/Game/Blueprints/Gameplay/Gameplay-GameMode` (`GameplayStatics.GetGameMode`)))
  (set `self.REFGameMode` _asgameplay__game_mode)
  (`KismetSystemLibrary.Delay` 0.5)
  (`self.Create Widgets`))

(event `Key|One`
  (params (Key :type "Key Structure"))
  (:`Pressed`
    (`/Game/Blueprints/Gameplay/Gameplay-GameMode.SpawnCharacter` (`self.REFGameMode`) self :!label _label)))

(event `Key|Gamepad_Special_Right`
  (params (Key :type "Key Structure"))
  (:`Pressed`
    (goto _label)))

(event `Key|Two`
  (params (Key :type "Key Structure"))
  (:`Pressed`
    (`/Game/Blueprints/Gameplay/Gameplay-GameMode.DespawnCharacter` (`self.REFGameMode`) self :!label _label_2)))

(event `Create Widgets`
  (bind _returnvalue (`|CreateWidget` "/Game/UI/Widgets/W_UltBar.W_UltBar_C" self))
  (set `self.UltBarP1` _returnvalue)
  (bind _returnvalue_2 (`|CreateWidget` "/Game/UI/Widgets/W_HealthBar.W_HealthBar_C" self))
  (set `self.HealthBarP1` _returnvalue_2)
  (bind _returnvalue_3 (`|CreateWidget` "/Game/UI/Widgets/W_HealthBarP2.W_HealthBarP2_C" self))
  (set `self.HealthBarP2` _returnvalue_3)
  (bind _returnvalue_4 (`|CreateWidget` "/Game/UI/Widgets/W_UltBarP2.W_UltBarP2_C" self))
  (set `self.UltBarP2` _returnvalue_4)
  (bind _returnvalue_5 (`|CreateWidget` "/Game/UI/Widgets/W_HealthBarP3.W_HealthBarP3_C" self))
  (set `self.HealthBarP3` _returnvalue_5)
  (bind _returnvalue_6 (`|CreateWidget` "/Game/UI/Widgets/W_UltBarP3.W_UltBarP3_C" self))
  (set `self.UltBarP3` _returnvalue_6)
  (bind _returnvalue_7 (`|CreateWidget` "/Game/UI/Widgets/W_HealthBarP4.W_HealthBarP4_C" self))
  (set `self.HealthBarP4` _returnvalue_7)
  (bind _returnvalue_8 (`|CreateWidget` "/Game/UI/Widgets/W_UltBarP4.W_UltBarP4_C" self))
  (set `self.UltBarP4` _returnvalue_8))

(event `Key|Gamepad_Special_Left`
  (params (Key :type "Key Structure"))
  (:`Pressed`
    (goto _label_2)))

(fn `UserConstructionScript`)